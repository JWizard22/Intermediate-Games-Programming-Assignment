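; BP_KillFloor is a kill-floor actor that shows a death menu when anything overlaps it.
; BeginPlay caches the first-person character, the PlayerStart location as a respawn point, and a pre-created UWB_DeathMenu widget.
; Overlap, with no check on the other actor, disables character input, pauses the game, and displays the menu with the mouse cursor.
; Teleport-to-respawn logic that restores input and unpauses is present but disconnected.
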(event `self.ReceiveBeginPlay`
  (bind _returnvalue (`GameplayStatics.GetActorOfClass` "/Game/FirstPerson/Blueprints/BP_FirstPersonCharacter.BP_FirstPersonCharacter_C"))
  (set `self.FirstPersonCharacter` _returnvalue)
  (bind _returnvalue_2 (`GameplayStatics.GetActorOfClass` "/Script/Engine.PlayerStart"))
  (bind _output_get (set `self.Respawn Point` (`self.K2_GetActorLocation` _returnvalue_2)))
  (bind _returnvalue_3 (`|CreateWidget` "/Game/Menus/UWB_DeathMenu.UWB_DeathMenu_C" (`GameplayStatics.GetPlayerController` 0)))
  (set `self.Death Menu` _returnvalue_3))

(event `self.ReceiveActorBeginOverlap`
  (params (OtherActor :type "Actor Object Reference"))
  (`KismetSystemLibrary.PrintString` "you fell")
  (`self.DisableInput` (`self.FirstPersonCharacter`) (`GameplayStatics.GetPlayerController` 0))
  (`GameplayStatics.SetGamePaused` true)
  (`UserWidget.AddToViewport` (`self.Death Menu`) 0)
  (set `PlayerController.bShowMouseCursor` true (`GameplayStatics.GetPlayerController` 0)))

(fn `UserConstructionScript`)