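; BP_WinShape is the goal actor that shows the win screen when BP_FirstPersonCharacter overlaps it.
; BeginPlay creates UWB_WinScreen in advance; the overlap adds it to the viewport, switches to UI-only input and shows the cursor.
; Tick rotates the actor toward a random target rotator by a step proportional to the remaining difference.
; SetRandomRotation picks a new target when the signed average of that difference drops below Speed.
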(event `self.ReceiveBeginPlay`
  (`self.SetRandomRotation`
    (:`Out`
      (bind _returnvalue (`|CreateWidget` "/Game/MainMenu/UWB_WinScreen.UWB_WinScreen_C"))
      (set `self.WinScreen` _returnvalue))))

(event `self.ReceiveActorBeginOverlap`
  (params (OtherActor :type "Actor Object Reference"))
  (bind _returnvalue (`GameplayStatics.GetPlayerController` 0))
  (cast `/Game/FirstPerson/Blueprints/BP_FirstPersonCharacter` OtherActor)
  (`WidgetBlueprintLibrary.SetInputMode_UIOnlyEx` _returnvalue null)
  (set `PlayerController.bShowMouseCursor` true _returnvalue)
  (`UserWidget.AddToViewport` (`self.WinScreen`) 0))

(event `self.ReceiveTick`
  (params (DeltaSeconds :type "Float (single-precision)"))
  (bind (_returnvalue_roll _returnvalue_pitch _returnvalue_yaw) (`KismetMathLibrary.BreakRotator` (`self.K2_GetActorRotation`)))
  (bind (_rdestination_roll _rdestination_pitch _rdestination_yaw) (`KismetMathLibrary.BreakRotator` (`self.RDestination`)))
  (bind (_rdistance_roll _rdistance_pitch _rdistance_yaw) (`KismetMathLibrary.BreakRotator` (`self.RDistance`)))
  (set `self.DeltaSeconds` DeltaSeconds)
  (set `self.RDistance` (`KismetMathLibrary.MakeRotator` (- _rdestination_roll _returnvalue_roll) (- _rdestination_pitch _returnvalue_pitch) (- _rdestination_yaw _returnvalue_yaw)))
  (set `self.RDirection` (`self.RDistance`))
  (set `self.RVelocity` (* (`self.RDirection`) (`self.Speed`)))
  (set `self.RStep` (* (`self.RVelocity`) (`self.DeltaSeconds`)))
  (`self.K2_AddActorWorldRotation` (`self.RStep`))
  (if (< (/ (+ _rdistance_roll _rdistance_pitch _rdistance_yaw) 3.0) (`self.Speed`))
    (`self.SetRandomRotation`)))

(fn `UserConstructionScript`)