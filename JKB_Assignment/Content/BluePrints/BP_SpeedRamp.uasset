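; Speed ramp actor that boosts the first-person character's max walk speed and acceleration while it overlaps the actor.
; BeginPlay caches the character's movement and camera components, and overlap begin and end switch between hardcoded boosted and normal values, with debug prints.
; Tick steps the camera FOV toward a wider target on entry and back at half that rate on exit, using fixed per-frame increments independent of delta time.
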(event `self.ReceiveBeginPlay`
  (bind _returnvalue (`GameplayStatics.GetActorOfClass` "/Game/FirstPerson/Blueprints/BP_FirstPersonCharacter.BP_FirstPersonCharacter_C"))
  (set `self.CharacterMovementComponent` (`Character.CharacterMovement` _returnvalue))
  (set `self.First Person CameraComponent` (`/Game/FirstPerson/Blueprints/BP_FirstPersonCharacter.FirstPersonCamera` _returnvalue)))

(event `self.ReceiveActorBeginOverlap`
  (params (OtherActor :type "Actor Object Reference"))
  (bind _charactermovementcomponent (`self.CharacterMovementComponent`))
  (cast `/Game/FirstPerson/Blueprints/BP_FirstPersonCharacter` OtherActor)
  (set `CharacterMovementComponent.MaxAcceleration` 2000.0 _charactermovementcomponent)
  (set `CharacterMovementComponent.MaxWalkSpeed` 3000.0 _charactermovementcomponent)
  (`KismetSystemLibrary.PrintString` "entered speed ramp")
  (set `self.target FOV` 105.0)
  (set `self.FOV Increasing` true))

(event `self.ReceiveActorEndOverlap`
  (params (OtherActor :type "Actor Object Reference"))
  (bind _charactermovementcomponent (`self.CharacterMovementComponent`))
  (cast `/Game/FirstPerson/Blueprints/BP_FirstPersonCharacter` OtherActor)
  (set `CharacterMovementComponent.MaxAcceleration` 1500.0 _charactermovementcomponent)
  (set `CharacterMovementComponent.MaxWalkSpeed` 2000.0 _charactermovementcomponent)
  (`KismetSystemLibrary.PrintString` "left speed ramp")
  (set `self.target FOV` 90.0)
  (set `self.FOV Increasing` false))

(event `self.ReceiveTick`
  (params (DeltaSeconds :type "Float (single-precision)"))
  (bind _first_person_cameracomponent (`self.First Person CameraComponent`))
  (if (`self.FOV Increasing`)
    (if (< (`self.current FOV`) (`self.target FOV`))
      (bind _output_get (set `self.current FOV` (+ (`self.current FOV`) 0.25)))
      (`CameraComponent.SetFieldOfView` _first_person_cameracomponent _output_get))
    (elif (> (`self.current FOV`) (`self.target FOV`))
      (bind _output_get_2 (set `self.current FOV` (- (`self.current FOV`) 0.125)))
      (`CameraComponent.SetFieldOfView` _first_person_cameracomponent _output_get_2))))

(fn `UserConstructionScript`)